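; BP_TagGiverArea is a placeable trigger zone that gives a configurable gameplay tag to actors while they overlap its box.
; Box overlap begin adds TagGiven to the actor as a loose, non-replicated tag, and overlap end removes it.
; The construction script sizes the box from BoxExtent with a fixed height and sets a text label showing the tag name.
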(event `self.Box.OnComponentBeginOverlap`
  (params (OverlappedComponent :type "PrimitiveComponent Object Reference") (OtherActor :type "Actor Object Reference") (OtherComp :type "PrimitiveComponent Object Reference") (OtherBodyIndex :type Integer) (bFromSweep :type Boolean) (SweepResult :type "HitResult Structure (by ref)"))
  (`AbilitySystemBlueprintLibrary.AddLooseGameplayTags` OtherActor (`BlueprintGameplayTagLibrary.MakeGameplayTagContainerFromArray` (`|MakeArray` (`self.TagGiven`)))))

(event `self.Box.OnComponentEndOverlap`
  (params (OverlappedComponent :type "PrimitiveComponent Object Reference") (OtherActor :type "Actor Object Reference") (OtherComp :type "PrimitiveComponent Object Reference") (OtherBodyIndex :type Integer))
  (`AbilitySystemBlueprintLibrary.RemoveLooseGameplayTags` OtherActor (`BlueprintGameplayTagLibrary.MakeGameplayTagContainerFromArray` (`|MakeArray` (`self.TagGiven`)))))

(fn `UserConstructionScript`
  (bind _boxextent (`self.BoxExtent`))
  (`BoxComponent.SetBoxExtent` (`self.Box`) (`KismetMathLibrary.MakeVector` _boxextent _boxextent 32.0) true)
  (`TextRenderComponent.K2_SetText` (`self.TextRender`) (`|FormatText` "TAG: {tagName}" (`BlueprintGameplayTagLibrary.GetTagName` (`self.TagGiven`)))))