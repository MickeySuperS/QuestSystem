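; Game mode that adds the game HUD and starts a quest through the NQuest subsystem.
; On BeginPlay it creates the WBP_Game widget, waits briefly, then creates and starts an instance of the Quest asset with itself as owner.
; Tick has the subsystem evaluate quests every frame.
; Debug print handlers for quest creation and quest, objective and condition completion exist, but their bindings are disconnected and never run.
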(event `CustomEvent`
  (params (QuestTags :type "GameplayTag Structure (by ref)"))
  (`KismetSystemLibrary.PrintText` (`|FormatText` "Qest Created: {tag}" (`BlueprintGameplayTagLibrary.GetTagName` QuestTags))))

(event `CustomEvent_1`
  (params (QuestTags :type "GameplayTag Structure (by ref)"))
  (`KismetSystemLibrary.PrintText` (`|FormatText` "Qest Completed: {tag}" (`BlueprintGameplayTagLibrary.GetTagName` QuestTags))))

(event `CustomEvent_3`
  (params (QuestTags :type "GameplayTag Structure (by ref)"))
  (`KismetSystemLibrary.PrintText` (`|FormatText` "Condition Completed: {tag}" (`BlueprintGameplayTagLibrary.GetTagName` QuestTags))))

(event `CustomEvent_2`
  (params (QuestTags :type "GameplayTag Structure (by ref)"))
  (`KismetSystemLibrary.PrintText` (`|FormatText` "Objective Completed: {tag}" (`BlueprintGameplayTagLibrary.GetTagName` QuestTags))))

(event `self.ReceiveBeginPlay`
  (bind _returnvalue (subsystem `NQuestSubsystem`))
  (bind _returnvalue_2 (`|CreateWidget` "/Game/UI/WBP_Game.WBP_Game_C" (`GameplayStatics.GetPlayerController` 0)))
  (`UserWidget.AddToViewport` _returnvalue_2 0)
  (`KismetSystemLibrary.Delay` 2.0)
  (`|ExecutionSequence`
    (:`then_1`
      (bind _returnvalue_3 (`NQuestSubsystem.CreateQuestInstance` _returnvalue self "/NoutQuest/Quest.Quest"))
      (`NQuestSubsystem.StartQuest` _returnvalue _returnvalue_3))))

(event `self.ReceiveTick`
  (params (DeltaSeconds :type "Float (single-precision)"))
  (`NQuestSubsystem.EvaluateQuests` (subsystem `NQuestSubsystem`)))

(fn `UserConstructionScript`)